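; Medium-tier asteroid Blueprint that merges with other mediums into a large asteroid and splits into two small ones on death.
; BeginPlay sets a force multiplier and keeps collision off for a short delay after spawning.
; On box overlap with another medium, DeletePriority picks one to handle the merge: it destroys itself and calls Collision on the other, which spawns the large asteroid in its place.
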(event `self.ReceiveBeginPlay`
  (`parent.ReceiveBeginPlay`)
  (set `self.ForceMultiplier` 5.0)
  (`self.SetActorEnableCollision` false)
  (`KismetSystemLibrary.Delay` 2.0)
  (`self.SetActorEnableCollision` true))

(event `self.Box.OnComponentBeginOverlap`
  (params (OverlappedComponent :type "PrimitiveComponent Object Reference") (OtherActor :type "Actor Object Reference") (OtherComp :type "PrimitiveComponent Object Reference") (OtherBodyIndex :type Integer) (bFromSweep :type Boolean) (SweepResult :type "HitResult Structure (by ref)"))
  ; Destroy an Asteroid OnCollision and Spawn a Bigger One
  (if (`self.ActorHasTag` OtherActor "Medium")
    (bind _asbp_asteroids_child_medium (cast `/Game/StickyAsteroids/Blueprints/Game/BP_Asteroids_Child_Medium` OtherActor))
    (if (< (`/Game/StickyAsteroids/Blueprints/Game/BP_AsteroidsBase.DeletePriority` _asbp_asteroids_child_medium) (`self.DeletePriority`))
      (`self.K2_DestroyActor`)
      (`self.Collision` _asbp_asteroids_child_medium))))

(fn `Collision`
  ; Collision Function Definition
  (`|SpawnActorFromClass` "/Game/StickyAsteroids/Blueprints/Game/BP_AsteroidsBase_Child_Large.BP_AsteroidsBase_Child_Large_C" (`KismetMathLibrary.MakeTransform` (.location (`SceneComponent.K2_GetComponentToWorld` (`self.SM_Asteroid`))) (.rotation (`SceneComponent.K2_GetComponentToWorld` (`self.SM_Asteroid`)))) "Undefined" "MultiplyWithRoot" null null)
  (`self.K2_DestroyActor`))

(fn `Death`
  (bind _returnvalue (`SceneComponent.K2_GetComponentToWorld` (`self.SM_Asteroid`)))
  ; Spawn 2 Small Asteroids on Death
  (`|SpawnActorFromClass` "/Game/StickyAsteroids/Blueprints/Game/BP_Asteroids_Child_Small.BP_Asteroids_Child_Small_C" _returnvalue "AdjustIfPossibleButAlwaysSpawn" "MultiplyWithRoot" null null)
  (`|SpawnActorFromClass` "/Game/StickyAsteroids/Blueprints/Game/BP_Asteroids_Child_Small.BP_Asteroids_Child_Small_C" _returnvalue "AdjustIfPossibleButAlwaysSpawn" "MultiplyWithRoot" null null)
  (`self.K2_DestroyActor`))

(fn `UserConstructionScript`
  (`parent.UserConstructionScript`))