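; Large asteroid enemy, a child Blueprint that splits into two medium asteroids when it dies.
; On BeginPlay it runs the parent logic and reports its spawn to the player's BP_Spaceship.
; Death spawns both medium asteroids around the mesh's transform, nudging the second further aside with a local offset.
; It then adds to the spaceship's score, reports the enemy death to it and destroys itself.
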(event `self.ReceiveBeginPlay`
  (`parent.ReceiveBeginPlay`)
  (bind _asbp_spaceship (cast `/Game/StickyAsteroids/Blueprints/Game/BP_Spaceship` (`GameplayStatics.GetPlayerPawn` 0)))
  (`/Game/StickyAsteroids/Blueprints/Game/BP_Spaceship.EnemySpawned` _asbp_spaceship))

(fn `Death`
  (bind _returnvalue (`SceneComponent.K2_GetComponentToWorld` (`self.SM_Asteroid`)))
  (bind _rotation (.rotation _returnvalue))
  (bind _scale (.scale _returnvalue))
  ; Spawn 2 Small Asteroids on Death
  (bind _returnvalue_2 (`|SpawnActorFromClass` "/Game/StickyAsteroids/Blueprints/Game/BP_Asteroids_Child_Medium.BP_Asteroids_Child_Medium_C" (`KismetMathLibrary.MakeTransform` (+ (.location _returnvalue) (`KismetMathLibrary.MakeVector` 4.0 4.0)) _rotation _scale) "AdjustIfPossibleButAlwaysSpawn" "MultiplyWithRoot" null null))
  (`self.K2_AddActorLocalOffset` _returnvalue_2 (0.0 0.0 0.0) false false)
  (bind _returnvalue_3 (`|SpawnActorFromClass` "/Game/StickyAsteroids/Blueprints/Game/BP_Asteroids_Child_Medium.BP_Asteroids_Child_Medium_C" (`KismetMathLibrary.MakeTransform` (+ (.location _returnvalue) (`KismetMathLibrary.MakeVector` -4.0 -4.0)) _rotation _scale) "AdjustIfPossibleButAlwaysSpawn" "MultiplyWithRoot" null null))
  (`self.K2_AddActorLocalOffset` _returnvalue_3 (-0.0 -250.0 0.0) false false)
  (bind _asbp_spaceship (cast `/Game/StickyAsteroids/Blueprints/Game/BP_Spaceship` (`GameplayStatics.GetPlayerPawn` 0)))
  (set `/Game/StickyAsteroids/Blueprints/Game/BP_Spaceship.Score` (+ (`/Game/StickyAsteroids/Blueprints/Game/BP_Spaceship.Score` _asbp_spaceship) 3) _asbp_spaceship)
  (bind _asbp_spaceship_2 (cast `/Game/StickyAsteroids/Blueprints/Game/BP_Spaceship` (`GameplayStatics.GetPlayerPawn` 0)))
  (`/Game/StickyAsteroids/Blueprints/Game/BP_Spaceship.EnemyDeath` _asbp_spaceship_2)
  (`self.K2_DestroyActor`))

(fn `UserConstructionScript`
  (`parent.UserConstructionScript`))