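; Player spaceship for an Asteroids-style game, steered with physics torque and thrust along the mesh's right vector.
; Shoot spawns bullets on both press and release, and Tick wraps the ship by negating its out-of-bounds X or Y.
; Touching an asteroid restarts the level, as does the enemy counter reaching zero, checked one second after a death.
; It also creates the score widget and toggles the pause menu on Escape.
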(event `InputAxis|Rotate`
  (params (AxisValue :type "Float (single-precision)"))
  ; Rotate Spaceship
  (`PrimitiveComponent.AddTorqueInDegrees` (`self.SM_Spaceship`) (`KismetMathLibrary.MakeVector` 0.0 0.0 (* AxisValue (`self.TorqueMultiplier`))) "None" true))

(event `InputAxis|MoveForward`
  (params (AxisValue :type "Float (single-precision)"))
  (bind _sm_spaceship (`self.SM_Spaceship`))
  ; Move Spaceship Forward
  (`PrimitiveComponent.AddForce` _sm_spaceship (* (* AxisValue (`self.ForceMultiplier`)) (`SceneComponent.GetRightVector` _sm_spaceship)) "None" true))

(event `InputAction|Shoot`
  (params (Key :type "Key Structure"))
  ; Spawn Bullet
  (:`Pressed`
    (`|SpawnActorFromClass` "/Game/StickyAsteroids/Blueprints/Game/BP_Bullet.BP_Bullet_C" (`SceneComponent.K2_GetComponentToWorld` (`self.BulletSpawnPoint`)) "AdjustIfPossibleButAlwaysSpawn" "MultiplyWithRoot" null null :!label _label))
  (:`Released`
    (goto _label)))

(event `self.ReceiveTick`
  (params (DeltaSeconds :type "Float (single-precision)"))
  (bind _x (.x (`SceneComponent.K2_GetComponentLocation` (`self.SM_Spaceship`))))
  (bind _y (.y (`SceneComponent.K2_GetComponentLocation` (`self.SM_Spaceship`))))
  ; Wrapping Screen
  (if (not (`KismetMathLibrary.InRange_FloatFloat` _x -4000.0 4000.0))
    (`SceneComponent.K2_SetWorldLocation` (`self.SM_Spaceship`) (`KismetMathLibrary.MakeVector` (* _x -1.0) (.y (`SceneComponent.K2_GetComponentLocation` (`self.SM_Spaceship`))) (.z (`SceneComponent.K2_GetComponentLocation` (`self.SM_Spaceship`)))) false false))
  (if (not (`KismetMathLibrary.InRange_FloatFloat` _y -7500.0 7500.0))
    (`SceneComponent.K2_SetWorldLocation` (`self.SM_Spaceship`) (`KismetMathLibrary.MakeVector` (.x (`SceneComponent.K2_GetComponentLocation` (`self.SM_Spaceship`))) (* _y -1.0) (.z (`SceneComponent.K2_GetComponentLocation` (`self.SM_Spaceship`)))) false false)))

(event `self.ReceiveBeginPlay`
  (bind _returnvalue (`|CreateWidget` "/Game/StickyAsteroids/Blueprints/Game/ScoreWidget.ScoreWidget_C"))
  (`UserWidget.AddToViewport` _returnvalue 0))

(event `self.Box.OnComponentBeginOverlap`
  (params (OverlappedComponent :type "PrimitiveComponent Object Reference") (OtherActor :type "Actor Object Reference") (OtherComp :type "PrimitiveComponent Object Reference") (OtherBodyIndex :type Integer) (bFromSweep :type Boolean) (SweepResult :type "HitResult Structure (by ref)"))
  (if (`self.ActorHasTag` OtherActor "Asteroid")
    (`KismetSystemLibrary.ExecuteConsoleCommand` "RestartLevel" null)))

(event `EnemySpawned`
  (set `self.EnemyCounter` (+ (`self.EnemyCounter`) 1)))

(event `EnemyDeath`
  (set `self.EnemyCounter` (- (`self.EnemyCounter`) 1))
  (`KismetSystemLibrary.Delay` 1.0)
  (if (<= (`self.EnemyCounter`) 0)
    (`KismetSystemLibrary.ExecuteConsoleCommand` "RestartLevel" null)))

(event `Key|Escape`
  (params (Key :type "Key Structure"))
  (bind _returnvalue (`GameplayStatics.GetPlayerController` 0))
  (:`Pressed`
    (if (not (`self.paused`))
      (set `self.paused` true)
      (bind _returnvalue_2 (`|CreateWidget` "/Game/StickyAsteroids/Blueprints/Game/PauseMenu.PauseMenu_C" _returnvalue))
      (bind _output_get (set `self.PauseMenuWidget` _returnvalue_2))
      (`UserWidget.AddToViewport` _output_get 0)
      (`WidgetBlueprintLibrary.SetInputMode_GameAndUIEx` _returnvalue (`self.PauseMenuWidget`))
      (set `PlayerController.bShowMouseCursor` true (`GameplayStatics.GetPlayerController` 0))
      (`GameplayStatics.SetGamePaused` true)
      (else
        (set `self.paused` false)
        (`Widget.RemoveFromParent` (`self.PauseMenuWidget`))
        (`GameplayStatics.SetGamePaused` false)
        (`WidgetBlueprintLibrary.SetInputMode_GameOnly` null)
        (set `PlayerController.bShowMouseCursor` false (`GameplayStatics.GetPlayerController` 0))))))

(fn `UserConstructionScript`)