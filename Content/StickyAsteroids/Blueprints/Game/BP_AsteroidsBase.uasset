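; Base asteroid actor that drifts across the play area and splits when it dies.
; BeginPlay rolls a random XY direction and a DeletePriority; Tick offsets the mesh along that direction by ForceMultiplier, without delta-time scaling.
; Each tick also wraps the mesh by negating out-of-bounds X or Y and reapplies actor scale from Medium or Large tags.
; Death spawns two medium child asteroids at the mesh's transform, then destroys the actor.
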(event `self.ReceiveBeginPlay`
  ; Create Random Direction Vector
  (set `self.RandomDirection` (`KismetMathLibrary.MakeVector` (`KismetMathLibrary.RandomFloatInRange` -1.0 1.0) (`KismetMathLibrary.RandomFloatInRange` -1.0 1.0)))
  (set `self.DeletePriority` (`KismetMathLibrary.RandomFloat`)))

(event `self.ReceiveTick`
  (params (DeltaSeconds :type "Float (single-precision)"))
  ; Move Asteroid
  (`SceneComponent.K2_AddWorldOffset` (`self.SM_Asteroid`) (* (`self.RandomDirection`) (`self.ForceMultiplier`)) false false)
  (`self.Wrapping`)
  (if (`self.ActorHasTag` "Medium")
    (`self.SetActorScale3D` (1.5 1.5 1.5))
    (elif (`self.ActorHasTag` "Large")
      (`self.SetActorScale3D` (2.0 2.0 2.0))
      (else
        (`self.SetActorScale3D` (1.0 1.0 1.0))))))

(fn `Death`
  (bind _returnvalue (`SceneComponent.K2_GetComponentToWorld` (`self.SM_Asteroid`)))
  ; Spawn 2 Medium Asteroids on Death
  (`|SpawnActorFromClass` "/Game/StickyAsteroids/Blueprints/Game/BP_Asteroids_Child_Medium.BP_Asteroids_Child_Medium_C" _returnvalue "AdjustIfPossibleButAlwaysSpawn" "MultiplyWithRoot" null null)
  (`|SpawnActorFromClass` "/Game/StickyAsteroids/Blueprints/Game/BP_Asteroids_Child_Medium.BP_Asteroids_Child_Medium_C" _returnvalue "AdjustIfPossibleButAlwaysSpawn" "MultiplyWithRoot" null null)
  (`self.K2_DestroyActor`))

(fn `UserConstructionScript`)

(fn `Wrapping`
  (bind _x (.x (`SceneComponent.K2_GetComponentLocation` (`self.SM_Asteroid`))))
  (bind _y (.y (`SceneComponent.K2_GetComponentLocation` (`self.SM_Asteroid`))))
  ; Wrapping Screen
  (if (not (`KismetMathLibrary.InRange_FloatFloat` _x -3900.0 3900.0))
    (`SceneComponent.K2_SetWorldLocation` (`self.SM_Asteroid`) (`KismetMathLibrary.MakeVector` (* _x -1.0) (.y (`SceneComponent.K2_GetComponentLocation` (`self.SM_Asteroid`))) (.z (`SceneComponent.K2_GetComponentLocation` (`self.SM_Asteroid`)))) false false))
  (if (not (`KismetMathLibrary.InRange_FloatFloat` _y -6300.0 6300.0))
    (`SceneComponent.K2_SetWorldLocation` (`self.SM_Asteroid`) (`KismetMathLibrary.MakeVector` (.x (`SceneComponent.K2_GetComponentLocation` (`self.SM_Asteroid`))) (* _y -1.0) (.z (`SceneComponent.K2_GetComponentLocation` (`self.SM_Asteroid`)))) false false)))