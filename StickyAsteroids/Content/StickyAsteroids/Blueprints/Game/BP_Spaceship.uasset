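; BP_Spaceship is the player-controlled ship in StickyAsteroids, which turns, thrusts and shoots from input.
; Rotate and MoveForward axes apply yaw torque and force to the SMSpaceship mesh as mass-independent acceleration, scaled by multiplier variables.
; Thrust follows the mesh's right vector as its forward direction.
; Pressing Shoot spawns a BP_Bullet at BulletSpawnPoint, adjusting for collisions but always spawning.
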(event `InputAxis|Rotate`
  (params (AxisValue :type "Float (single-precision)"))
  ; Rotate Spaceship
  (`PrimitiveComponent.AddTorqueInDegrees` (`self.SM_Spaceship`) (`KismetMathLibrary.MakeVector` 0.0 0.0 (* AxisValue (`self.TorqueMultiplier`))) "None" true))

(event `InputAxis|MoveForward`
  (params (AxisValue :type "Float (single-precision)"))
  (bind _sm_spaceship (`self.SM_Spaceship`))
  ; Move Spaceship Forward
  (`PrimitiveComponent.AddForce` _sm_spaceship (* (* AxisValue (`self.ForceMultiplier`)) (`SceneComponent.GetRightVector` _sm_spaceship)) "None" true))

(event `InputAction|Shoot`
  (params (Key :type "Key Structure"))
  ; Spawn Bullet
  (:`Pressed`
    (`|SpawnActorFromClass` "/Game/StickyAsteroids/Blueprints/Game/BP_Bullet.BP_Bullet_C" (`SceneComponent.K2_GetComponentToWorld` (`self.BulletSpawnPoint`)) "AdjustIfPossibleButAlwaysSpawn" "MultiplyWithRoot" null null)))

(fn `UserConstructionScript`)