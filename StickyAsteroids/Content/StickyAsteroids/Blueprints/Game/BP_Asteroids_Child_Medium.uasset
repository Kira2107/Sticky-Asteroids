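; Medium asteroid variant in Sticky Asteroids, a child Blueprint of a parent asteroid class.
; On BeginPlay it runs the parent logic, then sets its own ForceMultiplier.
; Its Death function spawns two small asteroid children at the mesh's world transform, adjusting for collisions but always spawning, then destroys itself.
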(event `self.ReceiveBeginPlay`
  (`parent.ReceiveBeginPlay`)
  (set `self.ForceMultiplier` 5.0))

(fn `Death`
  (bind _returnvalue (`SceneComponent.K2_GetComponentToWorld` (`self.SM_Asteroid`)))
  ; Spawn 2 Small Asteroids on Death
  (`|SpawnActorFromClass` "/Game/StickyAsteroids/Blueprints/Game/BP_Asteroids_Child_Small.BP_Asteroids_Child_Small_C" _returnvalue "AdjustIfPossibleButAlwaysSpawn" "MultiplyWithRoot" null null)
  (`|SpawnActorFromClass` "/Game/StickyAsteroids/Blueprints/Game/BP_Asteroids_Child_Small.BP_Asteroids_Child_Small_C" _returnvalue "AdjustIfPossibleButAlwaysSpawn" "MultiplyWithRoot" null null)
  (`self.K2_DestroyActor`))

(fn `UserConstructionScript`
  (`parent.UserConstructionScript`))