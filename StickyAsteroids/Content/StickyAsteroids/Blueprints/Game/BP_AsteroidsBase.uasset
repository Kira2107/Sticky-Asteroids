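; BP_AsteroidsBase is a base asteroid actor that drifts across the XY plane and splits when it dies.
; BeginPlay picks a random, unnormalized XY direction, and Tick offsets the SMAsteroid component along it by ForceMultiplier, without sweep or delta-time scaling.
; The Death function spawns two BP_Asteroids_Child_Medium actors at the mesh's world transform, then destroys the actor.
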(event `self.ReceiveBeginPlay`
  ; Create Random Direction Vector
  (set `self.RandomDirection` (`KismetMathLibrary.MakeVector` (`KismetMathLibrary.RandomFloatInRange` -1.0 1.0) (`KismetMathLibrary.RandomFloatInRange` -1.0 1.0) 0.0)))

(event `self.ReceiveTick`
  (params (DeltaSeconds :type "Float (single-precision)"))
  ; Move Asteroid
  (`SceneComponent.K2_AddWorldOffset` (`self.SM_Asteroid`) (* (`self.RandomDirection`) (`self.ForceMultiplier`)) false false))

(fn `Death`
  (bind _returnvalue (`SceneComponent.K2_GetComponentToWorld` (`self.SM_Asteroid`)))
  ; Spawn 2 Medium Asteroids on Death
  (`|SpawnActorFromClass` "/Game/StickyAsteroids/Blueprints/Game/BP_Asteroids_Child_Medium.BP_Asteroids_Child_Medium_C" _returnvalue "AdjustIfPossibleButAlwaysSpawn" "MultiplyWithRoot" null null)
  (`|SpawnActorFromClass` "/Game/StickyAsteroids/Blueprints/Game/BP_Asteroids_Child_Medium.BP_Asteroids_Child_Medium_C" _returnvalue "AdjustIfPossibleButAlwaysSpawn" "MultiplyWithRoot" null null)
  (`self.K2_DestroyActor`))

(fn `UserConstructionScript`)